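; Chest cover Blueprint that opens a treasure chest lid once two keys have been collected.
; ChestOpen increments a key counter and prints it.
; Interaction checks for exactly two keys, then plays a timeline that rolls the lid mesh up to -90 degrees.
; Otherwise it prints a French message saying both keys are needed.
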(event Custom|ChestOpen
  (Math|Integer|IncrementInt (Variables|Default|GetNumber%20of%20key)
    (:%20%20
      (Development|PrintString (Utilities|String|ToString(Integer) (Variables|Default|GetNumber%20of%20key))))))

(event EventInteraction
  (if (== (Variables|Default|GetNumber%20of%20key) 2)
    (bind _rotation (Timeline|OpenCHest Play)
      (:Update
        (Transformation|SetRelativeRotation (Variables|Default|GetStaticMeshComponent0) (Math|Rotator|MakeRotator (* _rotation -9e+01) 0.0 0.0) false false)))
    (else
      (Development|PrintString "il te faut les 2 clés"))))

(fn ConstructionScript)